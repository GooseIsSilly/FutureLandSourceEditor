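; BP_ItemPickup is a world pickup that displays a weapon and can be interacted with.
; On BeginPlay it spawns the weapon's Blueprint class at its capsule, turns off the weapon mesh's collision and attaches the weapon to itself.
; Projectile movement simulation is switched off at start, noted as a temporary workaround for a collision issue.
; Interaction fires once, destroying the pickup and spawned weapon without granting any item here.
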(event EventBeginPlay
  (Variables|/Script/Engine.ProjectileMovementComponent|SetbSimulationEnabled (Variables|Default|GetProjectileMovement) false) ; temp disabled due to collision issue
  (bind _returnvalue (Game|SpawnActorfromClass (Variables|/Game/Core/Weapons/WeaponIdentitys/BP_WeaponIdentity.BP_WeaponIdentity_C|GetWeaponBlueprint (Variables|Default|GetWeapon)) (Math|Transform|MakeTransform (Physics|GetCenterOfMass (Variables|Default|GetCapsuleCollision) "None") "0, 0, 0" "1.000000,1.000000,1.000000") "AlwaysSpawn" "MultiplyWithRoot" self 0.0 0))
  (Collision|SetCollisionEnabled (Variables|/Game/Core/Weapons/WeaponBlueprints/BP_WeaponBase.BP_WeaponBase_C|GetSkeletalMesh _returnvalue) "NoCollision")
  (bind _output_get (Variables|Default|SetWeaponActorRef _returnvalue))
  (Transformation|AttachActorToActor _output_get self "None" "SnapToTarget" "SnapToTarget" "KeepRelative" true))

(event EventInteraction
  (Utilities|FlowControl|DoOnce false
    (:Completed
      (Actor|DestroyActor)
      (Actor|DestroyActor (Variables|Default|GetWeaponActorRef)))))

(fn ConstructionScript)
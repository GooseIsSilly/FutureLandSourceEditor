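; Base weapon actor for a Character, handling equip, automatic fire, reload and dry fire with networked montages.
; Fire runs camera-based line traces through the owner's crosshair component, then applies damage, shooting effects, spread and camera shake.
; Montages replicate via server-to-multicast events, and their callbacks and notifies gate input and trigger reloads.
; Weapon name and timed "Hipfire" tags on the owner expose weapon state, while walk speed selects the spread profile.
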(event Custom|ApplyDamage_Multicast
  (params (DamagedActor :type Actor%20Object%20Reference) (BaseDamage :type Float%20%28single-precision%29) (EventInstigator :type Controller%20Object%20Reference) (DamageCauser :type Actor%20Object%20Reference) (DamageTypeClass :type Damage%20Type%20Class%20Reference))
  ;[0.15 0.15 0.15 0.5] Apply Damage
  (CallFunction|ApplyDamageServer DamagedActor BaseDamage EventInstigator DamageCauser DamageTypeClass))

(event Custom|ApplyDamage_Server
  (params (DamagedActor :type Actor%20Object%20Reference) (BaseDamage :type Float%20%28single-precision%29) (EventInstigator :type Controller%20Object%20Reference) (DamageCauser :type Actor%20Object%20Reference) (DamageTypeClass :type Damage%20Type%20Class%20Reference))
  ;[0.15 0.15 0.15 0.5] Apply Damage
  (Game|Damage|ApplyDamage DamagedActor BaseDamage EventInstigator DamageCauser DamageTypeClass))

(event Custom|RemoveTag_Multicast
  (params (Tag :type Name%20%28by%20ref%29))
  ;[1 1 1] Tags
  (Utilities|Array|RemoveItem (Variables|/Script/Engine.Actor|GetTags (Components|GetOwner)) Tag))

(event Custom|DelayRemoveTag
  (params (Duration :type Float%20%28single-precision%29) (Tag :type Name))
  ;[1 1 1] Tags
  (Utilities|FlowControl|RetriggerableDelay Duration)
  (Tools|RemoveTag Tag))

(event Custom|AddTag_Server
  (params (Tag :type Name%20%28by%20ref%29))
  ;[1 1 1] Tags
  (CallFunction|AddTagMulticast Tag))

(event Custom|RemoveTag_Server
  (params (Tag :type Name%20%28by%20ref%29))
  ;[1 1 1] Tags
  (CallFunction|RemoveTagMulticast Tag))

(event Custom|AddTag_Multicast
  (params (Tag :type Name%20%28by%20ref%29))
  ;[1 1 1] Tags
  (Utilities|Array|Add (Variables|/Script/Engine.Actor|GetTags (Components|GetOwner)) Tag))

(event EventDestroyed
  ;[1 1 1] Destroyed
  (Tools|RemoveTag (Variables|Config|GetWeaponName))
  (Tools|RemoveTag "Hipfire")
  (if (Tools|IsLocallyControlled)
    (Default|HideCrossHairs (Variables|Default|GetCT_Cmpt_Crosshair))
    (CallFunction|StopMontage (Tools|GetCharacterMesh) (Variables|Montage|GetCharacterEquipMontage))))

(event EventBeginPlay
  ;[1 1 1] Spawned
  (CallFunction|Init)
  (Utilities|FlowControl|Delay 0.5)
  (Development|SetHiddeninGame (Variables|Default|GetSkeletalMesh) false false))

(event Input|MouseEvents|LeftMouseButton
  (params (Key :type Key%20Structure))
  ;[1 1 1] Fire
  (:Pressed
    (bind _returnvalue (Utilities|Time|SetTimerbyEvent (EventDispatchers|CreateEvent :!event Fire) (Variables|Config|GetFire_Rate%20) true))
    (Action|Fire))
  (:Released
    (Utilities|Time|ClearandInvalidateTimerbyHandle _returnvalue)))

(event Input|KeyboardEvents|R
  (params (Key :type Key%20Structure))
  ;[1 1 1] Reload
  (:Pressed
    (Action|Reload)))

(event Custom|StopMontage
  (params (Mesh :type Skeletal%20Mesh%20Component%20Object%20Reference) (Montage :type Anim%20Montage%20Object%20Reference))
  (CallFunction|StopMontageServer Mesh Montage))

(event Custom|StopMontage_Multicast
  (params (Mesh :type Skeletal%20Mesh%20Component%20Object%20Reference) (Montage :type Anim%20Montage%20Object%20Reference))
  (bind _ascharacter (Utilities|Casting|CastToCharacter (Components|GetOwner Mesh)))
  (Animation|StopAnimMontage _ascharacter Montage))

(event Custom|PlayMontage_Multicast
  (params (TaskName :type Name) (Mesh :type Skeletal%20Mesh%20Component%20Object%20Reference) (Montage :type Anim%20Montage%20Object%20Reference) (SectionName :type Name))
  (bind _notifyname (Animation|Montage|PlayMontage Mesh Montage 1.0 0.0 SectionName)
    (:then
      (Montage|OnMontagePlayed TaskName SectionName))
    (:OnCompleted
      (Montage|OnMontageCompleted TaskName))
    (:OnBlendOut
      (Montage|OnMontageBlendOut TaskName))
    (:OnInterrupted
      (Montage|OnMontageInterrupted TaskName))
    (:OnNotifyBegin
      (Montage|OnMontageNotifyBegin TaskName _notifyname))
    (:OnNotifyEnd
      (Montage|OnMontageNotifyEnd TaskName _notifyname))))

(event Custom|StopMontage_Server
  (params (Mesh :type Skeletal%20Mesh%20Component%20Object%20Reference) (Montage :type Anim%20Montage%20Object%20Reference))
  (CallFunction|StopMontageMulticast Mesh Montage))

(event Custom|PlayMontage_Server
  (params (TaskName :type Name) (Mesh :type Skeletal%20Mesh%20Component%20Object%20Reference) (Montage :type Anim%20Montage%20Object%20Reference) (SectionName :type Name))
  (CallFunction|PlayMontageMulticast TaskName Mesh Montage SectionName))

(event Custom|PlayMontage
  (params (TaskName :type Name) (Mesh :type Skeletal%20Mesh%20Component%20Object%20Reference) (Montage :type Anim%20Montage%20Object%20Reference) (SectionName :type Name))
  (CallFunction|PlayMontageServer TaskName Mesh Montage SectionName))

(fn ConstructionScript)

(fn GetStartPoint
  (bind _returnvalue (Tools|GetCharacter))
  (bind _returnvalue_2 (Pawn|GetLocalViewingPlayerController _returnvalue))
  (bind _playercameramanager (Variables|/Script/Engine.PlayerController|GetPlayerCameraManager _returnvalue_2))
  (LocalVariables|SetLocal_Location (Camera|GetCameraLocation _playercameramanager))
  (LocalVariables|SetLocal_Rotation (Camera|GetCameraRotation _playercameramanager))
  (return (Math|Transform|MakeTransform (+ (LocalVariables|GetLocal_Location) (* (Math|Vector|GetForwardVector (LocalVariables|GetLocal_Rotation)) (Math|Vector|Distance(Vector) (LocalVariables|GetLocal_Location) (Transformation|GetActorLocation (Tools|GetCharacter))))) (LocalVariables|GetLocal_Rotation))))

(fn Fire
  (if (not (Variables|Default|GetDisableInput?))
    (if (>= (Variables|Config|GetAmmo) 0)
      (Math|Integer|DecrementInt (Variables|Config|GetAmmo)
        (:%20%20
          (CallFunction|PlayMontage "Fire" (Tools|GetCharacterMesh) (Variables|Montage|GetCharacterFireMontage) "None")
          (CallFunction|PlayMontage "None" (Variables|Default|GetSkeletalMesh) (Variables|Montage|GetWeaponFireMontage) "None")
          (Utilities|FlowControl|Sequence
            (:then_0
              (for _index (range 0 (- (Variables|Config|GetLineTraceCount) 1))
                (bind _hitresult (Crosshair|LineTrace))
                (CallFunction|ApplyDamageMulticast (.HitActor (Collision|BreakHitResult _hitresult)) (Variables|Config|GetDamage_Amount) 0 self)
                (Default|ShootEffect (Variables|Default|GetFireEffect) (Variables|Config|GetWeaponName) _hitresult)))
            (:then_1
              (Default|AddDynamicSpread (Variables|Default|GetCT_Cmpt_Crosshair) (Variables|Crosshair|GetFire_Spread) (Variables|Crosshair|GetFire_SpreadRecovery))
              (if (Tools|IsLocallyControlled)
                (Class|LegacyCameraShake|StartLegacyCameraShake (Variables|/Script/Engine.PlayerController|GetPlayerCameraManager (Pawn|GetLocalViewingPlayerController (Tools|GetCharacter))) "/Game/Core/Weapons/BP_CameraShake.BP_CameraShake_C" (Variables|Config|GetCameraShakeScale) "CameraLocal" "1.000000,1.000000,1.000000"))))))
      (else
        (CallFunction|PlayMontage "DryFire" (Tools|GetCharacterMesh) (Variables|Montage|GetCharacterDryFireMontage) "None")
        (Variables|Default|SetDisableInput? true)))))

(fn IsWalkMode
  (return (<= (Variables|/Script/Engine.CharacterMovementComponent|GetMaxWalkSpeed (Variables|/Script/Engine.Character|GetCharacterMovement (Tools|GetCharacter))) 2.5e+02)))

(fn LineTrace
  (bind _outhit (Default|LineTraceforObjects (Variables|Default|GetCT_Cmpt_Crosshair) (Crosshair|GetStartPoint) 1e+04 1.0 (Utilities|Array|MakeArray "ObjectTypeQuery3" "ObjectTypeQuery1" "ObjectTypeQuery2") false (Utilities|Array|MakeArray (Components|GetOwner) self 0) "None" true))
  (return _outhit))

(fn GetCharacterMesh
  (bind _ascharacter (Utilities|Casting|CastToCharacter (Components|GetOwner))
    (:then
      (return (Variables|/Script/Engine.Character|GetMesh _ascharacter)))
    (:CastFailed
      (return 0))))

(fn Reload
  (if (not (Variables|Default|GetDisableInput?))
    (Variables|Default|SetDisableInput? true)
    (Variables|Config|SetAmmo (Variables|Config|GetMaxAmmo))
    (CallFunction|PlayMontage "Reload" (Tools|GetCharacterMesh) (Variables|Montage|GetCharacterReloadMontage) "None")
    (CallFunction|PlayMontage "None" (Variables|Default|GetSkeletalMesh) (Variables|Montage|GetWeaponReloadMontage) "None")))

(fn AddTag
  (params (Tag :type Name))
  (CallFunction|AddTagServer Tag))

(fn RemoveTag
  (params (Tag :type Name))
  (bind _returnvalue (Components|GetOwner))
  (Utilities|IsValid _returnvalue
    (:Is%20Valid
      (Utilities|Array|RemoveItem (Variables|/Script/Engine.Actor|GetTags _returnvalue) Tag))))

(fn OnMontagePlayed
  (params (TaskName :type Name) (SectionName :type Name))
  (switch name TaskName
    (:Fire
      (if (not (CallFunction|IsWalkMode))
        (Tools|AddTag "Hipfire")
        (CallFunction|DelayRemoveTag 1.0 "Hipfire")))))

(fn OnMontageCompleted
  (params (TaskName :type Name)))

(fn OnMontageBlendOut
  (params (TaskName :type Name)))

(fn OnMontageInterrupted
  (params (TaskName :type Name))
  (switch name TaskName
    (:Reload
      _)
    (:DryFire
      _))
  (Variables|Default|SetDisableInput? false))

(fn OnMontageNotifyEnd
  (params (TaskName :type Name) (NotifyName :type Name))
  (switch name NotifyName
    (:DisableInput
      (Variables|Default|SetDisableInput? false))))

(fn OnMontageNotifyBegin
  (params (TaskName :type Name) (NotifyName :type Name))
  (switch name NotifyName
    (:TryReload
      (if (Tools|IsLocallyControlled)
        (Action|Reload)))
    (:DisableInput
      (Variables|Default|SetDisableInput? true))))

(fn GetCharacter
  (bind _ascharacter (Utilities|Casting|CastToCharacter (Components|GetOwner)))
  (return _ascharacter))

(fn IsLocallyControlled
  (bind _returnvalue (Tools|GetCharacter))
  (Utilities|IsValid _returnvalue
    (:Is%20Valid
      (return (Pawn|IsLocallyControlled _returnvalue)))))

(fn ResetSpread
  (if (CallFunction|IsWalkMode)
    (Default|SetDefaultSpread (Variables|Default|GetCT_Cmpt_Crosshair) (Variables|Crosshair|GetWalk_BaseSpread) (Variables|Crosshair|GetWalk_JumpSpread) (Variables|Crosshair|GetWalk_MovementSpread) (Variables|Crosshair|GetWalk_MaxSpread))
    (else
      (Default|SetDefaultSpread (Variables|Default|GetCT_Cmpt_Crosshair) (Variables|Crosshair|GetJog_BaseSpread) (Variables|Crosshair|GetJog_JumpSpread) (Variables|Crosshair|GetJog_MovementSpread) (Variables|Crosshair|GetJog_MaxSpread)))))

(fn Init
  (bind _returnvalue (Tools|GetCharacter))
  (Tools|AddTag (Variables|Config|GetWeaponName))
  (Utilities|FlowControl|Sequence
    (:then_0
      (if (Tools|IsLocallyControlled)
        (bind _output_get (Variables|Default|SetCT_Cmpt_Crosshair (Actor|GetComponentbyClass (Components|GetOwner) "/Game/Core/Player/Components/CT_Cmpt_Crosshair.CT_Cmpt_Crosshair_C")))
        (Utilities|IsValid _output_get
          (:Is%20Valid
            (Default|ShowCrossHairs (Variables|Default|GetCT_Cmpt_Crosshair))
            (EventDispatchers|BindEventtoOnTryResetSpread (Variables|Default|GetCT_Cmpt_Crosshair) (EventDispatchers|CreateEvent :!event ResetSpread))
            (Crosshair|ResetSpread)
            (Action|Equip)))))
    (:then_1
      (Networking|SwitchHasAuthority
        (:Authority
          (bind _returnvalue_2 (Game|SpawnActorfromClass "/Game/Core/Weapons/BP_ShootingEffect.BP_ShootingEffect_C" (Math|Transform|MakeTransform "0, 0, 0" "0, 0, 0" "1.000000,1.000000,1.000000") "Undefined" "MultiplyWithRoot" self 0))
          (Variables|Default|SetFireEffect _returnvalue_2))))
    (:then_2
      (Utilities|IsValid _returnvalue
        (:Is%20Valid
          (Input|EnableInput (Pawn|GetLocalViewingPlayerController _returnvalue)))))))

(fn Equip
  (CallFunction|PlayMontage "Equip" (Tools|GetCharacterMesh) (Variables|Montage|GetCharacterEquipMontage) "None"))
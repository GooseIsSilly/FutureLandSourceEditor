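; Lobby player controller that puts up the account creation screen and shows the mouse cursor.
; On BeginPlay, a local controller with an active WiFi connection spawns the W_CreateAccount widget and switches input to UI only; without WiFi no screen appears.
; A non-local controller on a dedicated server instead opens SkyfallMap with the listen option.
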(event Custom|SpawnHUD
  (bind _self self)
  (bind _returnvalue (UserInterface|CreateWidget "/Game/Widgets/Lobby/W_CreateAccount.W_CreateAccount_C" _self))
  (Input|SetInputModeUIOnly _self _returnvalue "DoNotLock" false)
  (UserInterface|Viewport|AddtoPlayerScreen _returnvalue))

(event EventBeginPlay
  (Variables|/Script/Engine.PlayerController|SetbShowMouseCursor self true)
  (if (Pawn|IsLocalController)
    (if (Class|MobilePatchingLibrary|HasActiveWiFiConnection)
      (CallFunction|SpawnHUD))
    (elif (Networking|IsDedicatedServer)
      (Game|OpenLevel(byObjectReference) "/Game/SkyfallMap.SkyfallMap" true "-listen"))))

(fn ConstructionScript)